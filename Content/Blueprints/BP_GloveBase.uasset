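; BP_GloveBase is a glove actor that shows punch feedback when its static mesh hits something.
; The construction script applies a red or blue material from GloveColor and sets the initial glow from DamageIntensity.
; On hit, BPPunchEffectComponent spawns an effect at the impact location, and SetDamageIntensity switches the GlowEnable material parameter on for two seconds.
; BeginPlay only prints a test string.
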(event OnComponentHit(StaticMesh)
  (params (HitComponent :type Primitive%20Component%20Object%20Reference) (OtherActor :type Actor%20Object%20Reference) (OtherComp :type Primitive%20Component%20Object%20Reference) (NormalImpulse :type Vector :default "0, 0, 0") (Hit :type Hit%20Result%20Structure%20%28by%20ref%29))
  (Default|SpawnPunchEffect (Variables|Default|GetBP_PunchEffectComponent) (.location Hit))
  (CallFunction|SetDamageIntensity 1.0)
  (Utilities|FlowControl|Delay 2.0)
  (CallFunction|SetDamageIntensity 0.0))

(event EventBeginPlay
  (Development|PrintString "TEST START"))

(event Collision|EventActorBeginOverlap
  (params (OtherActor :type Actor%20Object%20Reference)))

(event EventTick
  (params (DeltaSeconds :type Float%20%28single-precision%29)))

(fn ConstructionScript
  (switch Utilities|FlowControl|Switch|SwitchonEGloveColor (Variables|Default|GetGloveColor)
    (:NewEnumerator0
      (Rendering|Material|SetMaterial (Variables|Default|GetStaticMesh) 0 (Variables|Default|GetMIRed)))
    (:NewEnumerator1
      (Rendering|Material|SetMaterial (Variables|Default|GetStaticMesh) 0 (Variables|Default|GetMIBlue))))
  (CallFunction|SetDamageIntensity (Variables|Default|GetDamageIntensity)))

(fn SetDamageIntensity
  (params (DamageIntensity :type Float%20%28double-precision%29))
  (Rendering|Material|SetScalarParameterValueonMaterials (Variables|Default|GetStaticMesh) "GlowEnable" DamageIntensity))