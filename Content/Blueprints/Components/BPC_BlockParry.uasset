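; Component that lets a character block with either glove and parry an opponent's punch, stunning the incoming fist.
; Blocking swaps that arm collision's responses on two trace channels, and overlaps with another actor's glove are checked while blocking.
; Hits above an intensity threshold, from fist velocity or input, fire PunchBlocked and set a timed stun on the attacker's component, with glow and sound.
; Tick counts down stuns and draws optional debug spheres.
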(event Custom|CustomEvent
  (params (OverlappedComponent :type Primitive%20Component%20Object%20Reference) (OtherActor :type Actor%20Object%20Reference) (OtherComp :type Primitive%20Component%20Object%20Reference) (OtherBodyIndex :type Integer) (bFromSweep :type Boolean) (SweepResult :type Hit%20Result%20Structure%20%28by%20ref%29))
  (CallFunction|ProcessCollision (Variables|Default|GetbBlockingLeft) SweepResult OtherComp true))

(event Custom|CustomEvent_0
  (params (OverlappedComponent :type Primitive%20Component%20Object%20Reference) (OtherActor :type Actor%20Object%20Reference) (OtherComp :type Primitive%20Component%20Object%20Reference) (OtherBodyIndex :type Integer) (bFromSweep :type Boolean) (SweepResult :type Hit%20Result%20Structure%20%28by%20ref%29))
  (CallFunction|ProcessCollision (Variables|Default|GetbBlockingRight) SweepResult OtherComp false))

(event EventBeginPlay
  (bind _returnvalue (Components|GetOwner))
  (bind _output_get (Variables|Default|SetLeftArmCollision (Class|Actor|FindComponentbyTag _returnvalue "/Script/Engine.PrimitiveComponent" (Variables|Default|GetLeftArmBlockTag))))
  (Collision|SetCollisionEnabled _output_get "QueryAndPhysics")
  (bind _output_get_2 (Variables|Default|SetRightArmCollision (Class|Actor|FindComponentbyTag _returnvalue "/Script/Engine.PrimitiveComponent" (Variables|Default|GetRightArmBlockTag))))
  (Collision|SetCollisionEnabled _output_get_2 "QueryAndPhysics")
  (Utilities|FlowControl|Sequence
    (:then_0
      (Collision|BindEventtoOnComponentBeginOverlap (Variables|Default|GetLeftArmCollision) (delegate Custom|CustomEvent))
      (Collision|BindEventtoOnComponentBeginOverlap (Variables|Default|GetRightArmCollision) (delegate Custom|CustomEvent_0))
      (Variables|Default|SetPhysicsControl (Actor|GetComponentbyClass (Components|GetOwner) "/Script/PhysicsControl.PhysicsControlComponent"))
      (Variables|Default|SetPunchInput (Actor|GetComponentbyClass (Components|GetOwner) "/Game/Blueprints/Components/BPC_Input.BPC_Input_C")))))

(event EventTick
  (params (DeltaSeconds :type Float%20%28single-precision%29))
  (bind _leftarmcollision (Variables|Default|GetLeftArmCollision))
  (bind _rightarmcollision (Variables|Default|GetRightArmCollision))
  (Utilities|FlowControl|Sequence
    (:then_0
      (if (and (Variables|Default|GetbBlockingLeft) (Variables|Default|GetbDebug))
        (bind _assphere_collision (Utilities|Casting|CastToSphereComponent _leftarmcollision))
        (Rendering|Debug|DrawDebugSphere (Transformation|GetWorldLocation _leftarmcollision) (Variables|/Script/Engine.SphereComponent|GetSphereRadius _assphere_collision) 12 "(R=0.000000,G=1.000000,B=0.136755,A=1.000000)" 0.0)))
    (:then_1
      (if (and (Variables|Default|GetbBlockingRight) (Variables|Default|GetbDebug))
        (bind _assphere_collision_2 (Utilities|Casting|CastToSphereComponent _rightarmcollision))
        (Rendering|Debug|DrawDebugSphere (Transformation|GetWorldLocation _rightarmcollision) (Variables|/Script/Engine.SphereComponent|GetSphereRadius _assphere_collision_2) 12 "(R=0.999538,G=0.000000,B=1.000000,A=1.000000)" 0.0)))
    (:then_2
      (bind _output_get (Variables|Default|SetLeftStunTimer (- (Variables|Default|GetLeftStunTimer) DeltaSeconds)))
      (if (<= _output_get 0.0)
        (Variables|Default|SetLeftStunTimer 0.0)
        (Variables|Default|SetbLeftStunned false)))
    (:then_3
      (bind _output_get_2 (Variables|Default|SetRightStunTimer (- (Variables|Default|GetRightStunTimer) DeltaSeconds)))
      (if (<= _output_get_2 0.0)
        (Variables|Default|SetRightStunTimer 0.0)
        (Variables|Default|SetbRightStunned false)))))

(fn BlockArm
  (params (ArmCollision :type Primitive%20Component%20Object%20Reference) (PhysicsSet :type Name))
  (Collision|SetCollisionResponsetoChannel ArmCollision "ECC_GameTraceChannel2" "ECR_Ignore")
  (Collision|SetCollisionResponsetoChannel ArmCollision "ECC_GameTraceChannel1" "ECR_Overlap"))

(fn UnblockArm
  (params (ArmCollision :type Primitive%20Component%20Object%20Reference) (PhysicsSet :type Name))
  (Collision|SetCollisionResponsetoChannel ArmCollision "ECC_GameTraceChannel2" "ECR_Overlap")
  (Collision|SetCollisionResponsetoChannel ArmCollision "ECC_GameTraceChannel1" "ECR_Ignore"))

(fn SetBlockingLeft
  (params (Blocking :type Boolean))
  (bind _armleftphysicsset (Variables|Default|GetArmLeftPhysicsSet))
  (bind _leftarmcollision (Variables|Default|GetLeftArmCollision))
  (bind _output_get (Variables|Default|SetbBlockingLeft Blocking))
  (if _output_get
    (CallFunction|BlockArm _leftarmcollision _armleftphysicsset)
    (else
      (CallFunction|UnblockArm _leftarmcollision _armleftphysicsset))))

(fn SetBlockingRight
  (params (Blocking :type Boolean))
  (bind _armrightphysicsset (Variables|Default|GetArmRightPhysicsSet))
  (bind _rightarmcollision (Variables|Default|GetRightArmCollision))
  (bind _output_get (Variables|Default|SetbBlockingRight Blocking))
  (if _output_get
    (CallFunction|BlockArm _rightarmcollision _armrightphysicsset)
    (else
      (CallFunction|UnblockArm _rightarmcollision _armrightphysicsset))))

(fn ProcessCollision
  (params (IsBlocking :type Boolean) (HitResult :type Hit%20Result%20Structure) (OtherComponent :type Primitive%20Component%20Object%20Reference) (bLeft :type Boolean))
  (bind _returnvalue (Components|GetOwner OtherComponent))
  (bind _returnvalue_2 (CallFunction|IsValidBlockingCollision OtherComponent IsBlocking))
  (if _returnvalue_2
    (LocalVariables|SetHitIntensity (CallFunction|GetIntensity OtherComponent bLeft))
    (LocalVariables|SetIsOtherFistLeft (Components|ComponentHasTag OtherComponent "LeftArmBlock"))
    (bind _shouldstun (CallFunction|ShouldStun HitResult (LocalVariables|GetHitIntensity)))
    (if _shouldstun
      (Default|CallPunchBlocked (LocalVariables|GetHitIntensity) HitResult (LocalVariables|GetIsOtherFistLeft) bLeft _returnvalue)
      (CallFunction|StunFist (LocalVariables|GetIsOtherFistLeft) _returnvalue HitResult)
      ;[0.15 0.15 0.15 0.5] debug stunned fist
      (if (Variables|Default|GetbDebug)
        (bind _assphere_collision (Utilities|Casting|CastToSphereComponent OtherComponent))
        (Rendering|Debug|DrawDebugSphere (Transformation|GetWorldLocation OtherComponent) (Variables|/Script/Engine.SphereComponent|GetSphereRadius _assphere_collision) 12 "(R=0.630556,G=0.161575,B=1.000000,A=1.000000)" 2.0 2.0)))))

(fn StunFist
  (params (bLeft :type Boolean) (Actor :type Actor%20Object%20Reference) (HitResult :type Hit%20Result%20Structure))
  (bind _returnvalue (Actor|GetComponentbyClass Actor "BPC_BlockParry_C"))
  (bind _stuntime (Variables|Default|GetStunTime))
  (Utilities|FlowControl|Sequence
    (:then_0
      (if bLeft
        (Variables|BPC_BlockParry_C|SetbLeftStunned _returnvalue true)
        (Variables|BPC_BlockParry_C|SetLeftStunTimer _returnvalue _stuntime)
        (else
          (Variables|BPC_BlockParry_C|SetbRightStunned _returnvalue true)
          (Variables|BPC_BlockParry_C|SetRightStunTimer _returnvalue _stuntime))))
    (:then_1
      (bind _asbp_character_base (Utilities|Casting|CastToBP_Character_Base Actor))
      (if bLeft
        (Variables|/Game/Characters/Xob/BP_Character_Base.BP_Character_Base_C|SetLeftGlow _asbp_character_base 5e+01)
        (else
          (Variables|/Game/Characters/Xob/BP_Character_Base.BP_Character_Base_C|SetRightGlow _asbp_character_base 5e+01))))
    (:then_2
      (Audio|SpawnSound2D "/Game/Audio/sfx_parry.sfx_parry" 1.0 1.0 0.0 0))))

(fn ShouldStun
  (params (HitResult :type Hit%20Result%20Structure) (Intensity :type Float%20%28double-precision%29))
  (bind _returnvalue (> Intensity 0.5))
  (Utilities|FlowControl|Sequence
    (:then_0
      (if _returnvalue
        _))
    (:then_1
      (return _returnvalue))))

(fn GetIntensity
  (params (PrimitiveComponent :type Primitive%20Component%20Object%20Reference) (bLeftArm :type Boolean))
  (bind _returnvalue (Components|GetOwner PrimitiveComponent))
  (bind _returnvalue_2 (Actor|GetComponentbyClass _returnvalue "/Game/Blueprints/Components/BPC_Input.BPC_Input_C"))
  (bind _returnvalue_3 (Physics|GetPhysicsLinearVelocity PrimitiveComponent "None"))
  (return (Utilities|Select :Index (Variables|Default|GetIntensityMode) :NewEnumerator0 (Math|Float|Clamp(Float) (/ (Math|Vector|VectorLength _returnvalue_3) (Variables|Default|GetMaxFistSpeed))) :NewEnumerator1 (Math|Float|SelectFloat (Variables|/Game/Blueprints/Components/BPC_Input.BPC_Input_C|GetMaxIntensityLeft _returnvalue_2) (Variables|/Game/Blueprints/Components/BPC_Input.BPC_Input_C|GetMaxIntensityRight _returnvalue_2) bLeftArm))))

(fn IsValidBlockingCollision
  (params (OtherComponent :type Primitive%20Component%20Object%20Reference) (ThisGloveBlocking :type Boolean))
  (return (Math|Boolean|ANDBoolean (!= (Components|GetOwner OtherComponent) (Components|GetOwner)) (Components|ComponentHasTag OtherComponent "Glove") ThisGloveBlocking)))