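; Actor component that detects punches landing on other actors' heads and applies damage to them.
; On BeginPlay it finds the owner's left and right arm colliders by tag and binds their overlap events.
; Overlaps with another actor's Head-tagged component fire per-hand punch events carrying the hit and the hand's max intensity from BPC_Input.
; Damage scales linearly with that intensity; the hit result is currently unused in the calculation.
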(event Custom|OnComponentBeginOverlap_Event
  (params (OverlappedComponent :type Primitive%20Component%20Object%20Reference) (OtherActor :type Actor%20Object%20Reference) (OtherComp :type Primitive%20Component%20Object%20Reference) (OtherBodyIndex :type Integer) (bFromSweep :type Boolean) (SweepResult :type Hit%20Result%20Structure%20%28by%20ref%29))
  (bind _returnvalue (Components|GetOwner))
  (bind _returnvalue_2 (Actor|GetComponentbyClass _returnvalue "/Game/Blueprints/Components/BPC_Input.BPC_Input_C"))
  (bind _maxintensityleft (Variables|/Game/Blueprints/Components/BPC_Input.BPC_Input_C|GetMaxIntensityLeft _returnvalue_2))
  (if (and (!= OtherActor _returnvalue) (Components|ComponentHasTag OtherComp "Head"))
    (Development|PrintString (Utilities|String|ToString(Text) (Utilities|Text|FormatText "{owner}{comp} overlapped with {actor}.{otherComp}" _returnvalue OverlappedComponent OtherActor OtherComp)) false)
    (Default|CallLeftPunchEvent SweepResult OtherActor _maxintensityleft)
    (CallFunction|PunchActor OtherActor _maxintensityleft SweepResult)))

(event Custom|CustomEvent
  (params (OverlappedComponent :type Primitive%20Component%20Object%20Reference) (OtherActor :type Actor%20Object%20Reference) (OtherComp :type Primitive%20Component%20Object%20Reference) (OtherBodyIndex :type Integer) (bFromSweep :type Boolean) (SweepResult :type Hit%20Result%20Structure%20%28by%20ref%29))
  (bind _returnvalue (Components|GetOwner))
  (bind _returnvalue_2 (Actor|GetComponentbyClass _returnvalue "/Game/Blueprints/Components/BPC_Input.BPC_Input_C"))
  (bind _maxintensityright (Variables|/Game/Blueprints/Components/BPC_Input.BPC_Input_C|GetMaxIntensityRight _returnvalue_2))
  (if (and (!= OtherActor _returnvalue) (Components|ComponentHasTag OtherComp "Head"))
    (Default|CallRightPunchEvent SweepResult OtherActor _maxintensityright)
    (CallFunction|PunchActor OtherActor _maxintensityright SweepResult)))

(event EventBeginPlay
  (Variables|Default|SetLeftCollision (Class|Actor|FindComponentbyTag (Components|GetOwner) "/Script/Engine.PrimitiveComponent" (Variables|Components|GetLeftArmBlockTag)))
  (Variables|Default|SetRightCollision (Class|Actor|FindComponentbyTag (Components|GetOwner) "/Script/Engine.PrimitiveComponent" (Variables|Components|GetRightArmBlockTag)))
  (Collision|AssignOnComponentBeginOverlap (Variables|Default|GetLeftCollision) (delegate Custom|OnComponentBeginOverlap_Event))
  (Collision|AssignOnComponentBeginOverlap (Variables|Default|GetRightCollision) (delegate Custom|CustomEvent)))

(event EventTick
  (params (DeltaSeconds :type Float%20%28single-precision%29)))

(fn PunchActor
  (params (PunchedActor :type Actor%20Object%20Reference) (Intensity :type Float%20%28double-precision%29) (HitResult :type Hit%20Result%20Structure))
  (Utilities|IsValid PunchedActor
    (:Is%20Valid
      (Game|Damage|ApplyDamage PunchedActor (CallFunction|CalculateDamage Intensity HitResult) 0 0 "/Script/Engine.DamageType"))))

(fn CalculateDamage
  (params (Intensity :type Float%20%28double-precision%29) (HitResult :type Hit%20Result%20Structure))
  (return (* Intensity 1e+01)))