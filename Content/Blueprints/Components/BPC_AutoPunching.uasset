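; Actor component that generates automatic, alternating punch motion values for its owner's two arms.
; BeginPlay caches world transforms of the primitive components tagged LeftArmBlock and RightArmBlock.
; While enabled, Tick derives right and left alphas from absolute sine and cosine of game time scaled by PunchSpeed, otherwise zeroing them.
; GetPunchingParams exposes alphas and cached transforms; unconnected nodes hold an unused PunchDistance offset and debug sphere.
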(event EventBeginPlay
  (bind _returnvalue (Components|GetOwner))
  (Variables|Default|SetLeftArmIdleTransform (Transformation|GetWorldTransform (Class|Actor|FindComponentbyTag _returnvalue "/Script/Engine.PrimitiveComponent" "LeftArmBlock")))
  (Variables|Default|SetRightArmIdleTransform (Transformation|GetWorldTransform (Class|Actor|FindComponentbyTag _returnvalue "/Script/Engine.PrimitiveComponent" "RightArmBlock"))))

(event EventTick
  (params (DeltaSeconds :type Float%20%28single-precision%29))
  (bind _returnvalue (Utilities|Time|GetGameTimeinSeconds))
  (bind _punchspeed (Variables|Default|GetPunchSpeed))
  (bind _returnvalue_2 (* _returnvalue _punchspeed))
  (if (Variables|Default|GetbEnabled)
    (Variables|Default|SetRightAlpha (Math|Float|Absolute(Float) (Math|Trig|Sin(Radians) _returnvalue_2)))
    (Variables|Default|SetLeftAlpha (Math|Float|Absolute(Float) (Math|Trig|Cos(Radians) _returnvalue_2)))
    (else
      (Variables|Default|SetLeftAlpha 0.0)
      (Variables|Default|SetRightAlpha 0.0))))

(fn GetPunchingParams
  (return (Variables|Default|GetRightAlpha) (Variables|Default|GetLeftAlpha) (Variables|Default|GetRightArmIdleTransform) (Variables|Default|GetLeftArmIdleTransform)))