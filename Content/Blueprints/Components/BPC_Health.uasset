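; BPC_Health is a component for BP_Character_Base owners that applies damage and creates the player HUD.
; On BeginPlay it binds to the owner's OnTakeAnyDamage, subtracts damage from the character's own Health variable and only prints a debug message at zero or below.
; AddHUD creates WBP_PlayerHUD for the owner's PlayerController and adds it to that player's screen; nothing here calls it, and OnPawnPossessed is empty.
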(event Custom|OnDamageTaken
  (params (DamagedActor :type Actor%20Object%20Reference) (Damage :type Float%20%28single-precision%29) (DamageType :type Damage%20Type%20Object%20Reference) (InstigatedBy :type Controller%20Object%20Reference) (DamageCauser :type Actor%20Object%20Reference))
  (Variables|/Game/Characters/Xob/BP_Character_Base.BP_Character_Base_C|SetHealth (Variables|Default|GetCharacterBase) (- (Variables|/Game/Characters/Xob/BP_Character_Base.BP_Character_Base_C|GetHealth (Variables|Default|GetCharacterBase)) Damage))
  (if (<= (Variables|/Game/Characters/Xob/BP_Character_Base.BP_Character_Base_C|GetHealth (Variables|Default|GetCharacterBase)) 0.0)
    (Development|PrintString "MUERTISIMO")))

(event Custom|AddHUD
  (params (ControllerRef :type Controller%20Object%20Reference))
  (Utilities|IsValid (Pawn|GetControlledPawn ControllerRef)
    (:Is%20Valid
      (bind _asbp_character_base (Utilities|Casting|CastToBP_Character_Base (Components|GetOwner)))
      (bind _asplayer_controller (Utilities|Casting|CastToPlayerController (Pawn|GetController _asbp_character_base)))
      (bind _returnvalue (UserInterface|CreateWidget "/Game/Blueprints/Widgets/WBP_PlayerHUD.WBP_PlayerHUD_C" _asplayer_controller))
      (bind _output_get (Variables|Default|SetHealthBarWidget _returnvalue))
      (UserInterface|Viewport|AddtoPlayerScreen _output_get))))

(event EventTick
  (params (DeltaSeconds :type Float%20%28single-precision%29)))

(event EventBeginPlay
  (bind _asbp_character_base (Utilities|Casting|CastToBP_Character_Base (Components|GetOwner)))
  (bind _output_get (Variables|Default|SetCharacterBase _asbp_character_base))
  (EventDispatchers|BindEventtoOnTakeAnyDamage _output_get (delegate Custom|OnDamageTaken)))

(fn OnPawnPossessed
  (params (ControllerRef :type Controller%20Object%20Reference)))