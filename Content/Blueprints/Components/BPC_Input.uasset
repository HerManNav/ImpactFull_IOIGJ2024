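; Character input component that turns thumbstick and block input into fist targets and blocking state for melee combat.
; Each Tick tracks hand sockets as idle positions; each stick offsets its fist in world XY, scaled by arm length and single components of the actor's forward/right vectors.
; Block inputs set flags and notify BPC_BlockParry.
; Getters expose fist transforms, punch alphas and block values; BindInput adds the player mapping context.
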(event Input|EnhancedActionEvents|EnhancedInputActionIA_RightStick_Move
  (params (ActionValue :type Vector%202D%20Structure) (ElapsedSeconds :type Float%20%28double-precision%29) (TriggeredSeconds :type Float%20%28double-precision%29) (InputAction :type Input%20Action%20Object%20Reference :default "/Game/Input/IA_RightStick_Move.IA_RightStick_Move"))
  (bind (_x _y) (Math|Vector2D|BreakVector2D ActionValue))
  ;[0.15 0.15 0.15 0.5] Fists movement
  (:Triggered
    (if (> _y (Variables|Default|GetMaxBack))
      (Variables|Exposed|SetRightAlpha (Math|Vector2D|Vector2DLength ActionValue))
      (Variables|Default|SetRighMoving true)
      (bind (_plane_x _plane_y) (CallFunction|FromJoysticktoXYPlane _x _y))
      (Variables|Exposed|SetRightFist (Math|Transform|MakeTransform (+ (.location (Variables|Default|GetRightFistIdle)) (Math|Vector|MakeVector _plane_x _plane_y 0.0)) "0, 0, 0" "1.000000,1.000000,1.000000"))
      (else
        (Variables|Exposed|SetRightFist (Variables|Default|GetRightFistIdle) :!label _label)
        (Variables|Default|SetRighMoving false)
        (Variables|Exposed|SetRightAlpha 0.0))))
  (:Completed
    (goto _label)))

(event Input|EnhancedActionEvents|EnhancedInputActionIA_LeftStick_Move
  (params (ActionValue :type Vector%202D%20Structure) (ElapsedSeconds :type Float%20%28double-precision%29) (TriggeredSeconds :type Float%20%28double-precision%29) (InputAction :type Input%20Action%20Object%20Reference :default "/Game/Input/IA_LeftStick_Move.IA_LeftStick_Move"))
  (bind (_x _y) (Math|Vector2D|BreakVector2D ActionValue))
  ;[0.15 0.15 0.15 0.5] Fists movement
  (:Triggered
    (if (> _y (Variables|Default|GetMaxBack))
      (Variables|Exposed|SetLeftAlpha (Math|Vector2D|Vector2DLength ActionValue))
      (Variables|Default|SetLeftMoving true)
      (bind (_plane_x _plane_y) (CallFunction|FromJoysticktoXYPlane _x _y))
      (Variables|Exposed|SetLeftFist (Math|Transform|MakeTransform (+ (.location (Variables|Default|GetLeftFistIdle)) (Math|Vector|MakeVector _plane_x _plane_y 0.0)) "0, 0, 0" "1.000000,1.000000,1.000000"))
      (else
        (Variables|Exposed|SetLeftFist (Variables|Default|GetLeftFistIdle) :!label _label)
        (Variables|Default|SetLeftMoving false)
        (Variables|Exposed|SetLeftAlpha 0.0))))
  (:Completed
    (goto _label)))

(event Input|EnhancedActionEvents|EnhancedInputActionIA_BlockRight
  (params (ActionValue :type Boolean) (ElapsedSeconds :type Float%20%28double-precision%29) (TriggeredSeconds :type Float%20%28double-precision%29) (InputAction :type Input%20Action%20Object%20Reference :default "/Game/Input/IA_BlockRight.IA_BlockRight"))
  (bind _blockparrycomponent (Variables|Default|GetBlockParryComponent))
  ;[0.15 0.15 0.15 0.5] Block/Parry
  (:Started
    (Default|SetBlockingRight _blockparrycomponent true)
    (Variables|Default|SetBlockingRight true))
  (:Completed
    (Default|SetBlockingRight _blockparrycomponent false)
    (Variables|Default|SetBlockingRight false)))

(event Input|EnhancedActionEvents|EnhancedInputActionIA_BlockLeft
  (params (ActionValue :type Boolean) (ElapsedSeconds :type Float%20%28double-precision%29) (TriggeredSeconds :type Float%20%28double-precision%29) (InputAction :type Input%20Action%20Object%20Reference :default "/Game/Input/IA_BlockLeft.IA_BlockLeft"))
  (bind _blockparrycomponent (Variables|Default|GetBlockParryComponent))
  ;[0.15 0.15 0.15 0.5] Block/Parry
  (:Started
    (Default|SetBlockingLeft _blockparrycomponent true)
    (Variables|Default|SetBlockingLeft true))
  (:Completed
    (Default|SetBlockingLeft _blockparrycomponent false)
    (Variables|Default|SetBlockingLeft false)))

(event EventBeginPlay
  (Utilities|FlowControl|Sequence
    (:then_0
      (bind _output_get (Variables|Default|SetOwner (Components|GetOwner)))
      (bind _ascharacter (Utilities|Casting|CastToCharacter _output_get))
      (Variables|Default|SetCharacter _ascharacter)
      (Variables|Default|SetBlockParryComponent (Actor|GetComponentbyClass _output_get "/Game/Blueprints/Components/BPC_BlockParry.BPC_BlockParry_C")))
    (:then_1
      ;[0.15 0.15 0.15 0.5] Init Right Fist
      (bind _output_get_2 (Variables|Default|SetRightFistIdle (Math|Transform|MakeTransform (.location (Transformation|GetSocketTransform (Variables|/Script/Engine.Character|GetMesh (Variables|Default|GetCharacter)) "hand_r" "RTS_World")) "0, 0, 0" "1.000000,1.000000,1.000000")))
      (Variables|Exposed|SetRightFist _output_get_2)
      ;[0.15 0.15 0.15 0.5] Init Left Fist
      (bind _output_get_3 (Variables|Default|SetLeftFistIdle (Math|Transform|MakeTransform (.location (Transformation|GetSocketTransform (Variables|/Script/Engine.Character|GetMesh (Variables|Default|GetCharacter)) "hand_l" "RTS_World")) "0, 0, 0" "1.000000,1.000000,1.000000")))
      (Variables|Exposed|SetLeftFist _output_get_3))))

(event EventTick
  (params (DeltaSeconds :type Float%20%28single-precision%29))
  (Utilities|FlowControl|Sequence
    (:then_0
      (if (Variables|Debug|GetDrawDebug)
        (Rendering|Debug|DrawDebugSphere (.location (Variables|Exposed|GetRightFist)) 1e+01 12 "(R=1.000000,G=0.000000,B=0.072148,A=1.000000)" 0.0 1.0)
        (Rendering|Debug|DrawDebugSphere (.location (Variables|Exposed|GetLeftFist)) 1e+01 12 "(R=0.000000,G=0.044825,B=0.897916,A=1.000000)" 0.0 1.0)))
    (:then_1
      (bind _output_get (Variables|Default|SetRightFistIdle (Transformation|GetSocketTransform (Variables|/Script/Engine.Character|GetMesh (Variables|Default|GetCharacter)) "hand_r" "RTS_World")))
      (if (not (Variables|Default|GetRighMoving))
        (Variables|Exposed|SetRightFist _output_get)))
    (:then_2
      (bind _output_get_2 (Variables|Default|SetLeftFistIdle (Transformation|GetSocketTransform (Variables|/Script/Engine.Character|GetMesh (Variables|Default|GetCharacter)) "hand_l" "RTS_World")))
      (if (not (Variables|Default|GetLeftMoving))
        (Variables|Exposed|SetLeftFist _output_get_2)))))

(fn BindInput
  (params (Object :type Controller%20Object%20Reference))
  (bind _asplayer_controller (Utilities|Casting|CastToPlayerController Object))
  (Input|AddMappingContext (PlayerController|LocalPlayerSubsystems|GetEnhancedInputLocalPlayerSubsystem _asplayer_controller) "/Game/Input/IMC_Player.IMC_Player" 0 "(bIgnoreAllPressedKeysUntilRelease=True,bForceImmediately=False,bNotifyUserSettings=False)"))

(fn FromJoysticktoXYPlane
  (params (Joystick_X :type Float%20%28double-precision%29) (Joystick_Y :type Float%20%28double-precision%29))
  (bind _owner (Variables|Default|GetOwner))
  (bind _maxarmlength (Variables|Default|GetMaxArmLength))
  (return (* Joystick_Y (.x (Transformation|GetActorForwardVector _owner)) _maxarmlength) (* Joystick_X (.y (Transformation|GetActorRightVector _owner)) _maxarmlength)))

(fn GetBlockingParams
  (return (Math|Conversions|ToFloat(Boolean) (Variables|Default|GetBlockingLeft)) (Math|Conversions|ToFloat(Boolean) (Variables|Default|GetBlockingRight))))

(fn GetPunchingParams
  (return (Variables|Exposed|GetRightAlpha) (Variables|Exposed|GetLeftAlpha) (Variables|Exposed|GetRightFist) (Variables|Exposed|GetLeftFist)))