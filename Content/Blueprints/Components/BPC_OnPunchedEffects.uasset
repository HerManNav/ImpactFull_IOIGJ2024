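; Actor component that plays impact feedback when its owner lands a punch.
; On BeginPlay it binds to the left and right punch events of the owner's BPC_PunchDetectionComponent, with both hands sharing one effects path.
; Punches at or above the hard threshold play a hard sound at the hit location and a world camera shake at the owner; weaker ones play a soft sound.
; No particles are spawned.
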(event Custom|LeftPunchEffects
  (params (PunchHitResult :type Hit%20Result%20Structure) (PunchedActor :type Actor%20Object%20Reference) (PunchIntensity :type Float%20%28double-precision%29))
  ;[0.15 0.15 0.15 0.5] Spawn sounds and particles
  (if (>= PunchIntensity (Variables|Default|GetHardPunchThreshold))
    (Audio|SpawnSoundatLocation "/Game/Audio/Raw/punch_hard.punch_hard" (.location PunchHitResult) "0, 0, 0" 1.0 1.0 0.0 0 0)
    (Camera|PlayWorldCameraShake "/Game/Blueprints/VFX/BP_CameraShake.BP_CameraShake_C" (Transformation|GetActorLocation (Components|GetOwner)) 0.0 1e+05)
    (else
      (Audio|SpawnSoundatLocation "/Game/Audio/Raw/punch_soft.punch_soft" (.location PunchHitResult) "0, 0, 0" 1.0 1.0 0.0 0 0))))

(event Custom|RightPunchEffects
  (params (PunchHit :type Hit%20Result%20Structure) (PunchedActor :type Actor%20Object%20Reference) (PunchIntensity :type Float%20%28double-precision%29))
  ;[0.15 0.15 0.15 0.5] Spawn sounds and particles
  (if (>= (stale Custom|LeftPunchEffects PunchIntensity) (Variables|Default|GetHardPunchThreshold))
    (Audio|SpawnSoundatLocation "/Game/Audio/Raw/punch_hard.punch_hard" (.location (stale Custom|LeftPunchEffects PunchHitResult)) "0, 0, 0" 1.0 1.0 0.0 0 0)
    (Camera|PlayWorldCameraShake "/Game/Blueprints/VFX/BP_CameraShake.BP_CameraShake_C" (Transformation|GetActorLocation (Components|GetOwner)) 0.0 1e+05)
    (else
      (Audio|SpawnSoundatLocation "/Game/Audio/Raw/punch_soft.punch_soft" (.location (stale Custom|LeftPunchEffects PunchHitResult)) "0, 0, 0" 1.0 1.0 0.0 0 0))))

(event EventBeginPlay
  (bind _returnvalue (Components|GetOwner))
  (bind _returnvalue_2 (Actor|GetComponentbyClass _returnvalue "/Game/Blueprints/Components/BPC_PunchDetectionComponent.BPC_PunchDetectionComponent_C"))
  (EventDispatchers|BindEventtoLeftPunchEvent _returnvalue_2 (delegate Custom|LeftPunchEffects))
  (EventDispatchers|BindEventtoRightPunchEvent _returnvalue_2 (delegate Custom|RightPunchEffects)))

(event EventTick
  (params (DeltaSeconds :type Float%20%28single-precision%29)))